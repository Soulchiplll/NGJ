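; theWall_BP is a wall actor whose cube material reacts to the position of the player's ball.
; On BeginPlay it creates a dynamic material instance from the Core material and applies it to the Cube mesh.
; Every tick it writes the world location of ThePlayer's TheBall into the material's "Loca" vector parameter, leaving any visual effect to the shader.
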(event `self.ReceiveBeginPlay`
  (bind _returnvalue (`KismetMaterialLibrary.CreateDynamicMaterialInstance` "/Game/_hl/_HL/Mat/core.core"))
  (bind _output_get (set `self.theMat` _returnvalue))
  (`PrimitiveComponent.SetMaterial` (`self.Cube`) 0 _output_get))

(event `self.ReceiveTick`
  (params (DeltaSeconds :type "Float (single-precision)"))
  (`MaterialInstanceDynamic.SetVectorParameterValue` (`self.theMat`) "Loca" (`KismetMathLibrary.Conv_VectorToLinearColor` (`SceneComponent.K2_GetComponentLocation` (`gameBall.theBall` (`self.thePlayer`))))))

(fn `UserConstructionScript`)