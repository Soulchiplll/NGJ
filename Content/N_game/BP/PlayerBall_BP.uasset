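; Player ball pawn that handles input, starts the ball spawner on first Bottom press, calls Round while held, and toggles a board widget with Tab.
; Losing the shield expands and fades the TheEternal mesh as a shockwave that repels and breaks nearby OtherBall actors; SheildBack restores it.
; Tick drives that effect and eases the Cherger component, reattaching it to the chosen ball or itself.
; Impacts and shield breaks shake the camera.
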(event `self.ReceiveBeginPlay`
  (`self.start`))

(event `EnhancedInput|/Game/N_game/input/tab`
  (params (ActionValue :type Boolean) (ElapsedSeconds :type "Float (double-precision)") (TriggeredSeconds :type "Float (double-precision)") (InputAction :type "InputAction Object Reference" :default "/Game/N_game/input/tab.tab"))
  (bind _theboard (`self.theBoard`))
  (:`Started`
    (set `/Game/N_game/UI/theBoard.isVising` (not (`/Game/N_game/UI/theBoard.isVising` _theboard)) _theboard)))

(event `self.ReceiveTick`
  (params (DeltaSeconds :type "Float (single-precision)"))
  (`self.SheildProcess` DeltaSeconds)
  (`self.ChosenCheck`)
  (set `self.LightComp` (`self.DirectionalLight`))
  (`KismetSystemLibrary.PrintText` (`KismetTextLibrary.Conv_IntToText` (`KismetArrayLibrary.Array_Length` (`self.otherBalls`)))))

(event `EnhancedInput|/Game/N_game/input/Bottom`
  (params (ActionValue :type Boolean) (ElapsedSeconds :type "Float (double-precision)") (TriggeredSeconds :type "Float (double-precision)") (InputAction :type "InputAction Object Reference" :default "/Game/N_game/input/Bottom.Bottom"))
  (:`Triggered`
    (`self.Round`))
  (:`Started`
    (if (not (`self.isFirstSpace`))
      (set `self.isFirstSpace` true)
      (bind _outactors (`GameplayStatics.GetAllActorsOfClass` "/Game/N_game/BP/BallSpawner_BP.BallSpawner_BP_C"))
      (set `BallSpawner.isStarted` true (`|GetArrayItem` _outactors)))
    (set `self.isRounding` true))
  (:`Completed`
    (set `self.isRounding` false)))

(event `self.Sphere.OnComponentHit`
  (params (HitComponent :type "PrimitiveComponent Object Reference") (OtherActor :type "Actor Object Reference") (OtherComp :type "PrimitiveComponent Object Reference") (NormalImpulse :type "Vector Structure") (Hit :type "HitResult Structure (by ref)"))
  (`LegacyCameraShake.StartLegacyCameraShake` (`GameplayStatics.GetPlayerCameraManager` 0) "/Game/N_game/other/thesShake.thesShake_C" (/ (`KismetMathLibrary.Sqrt` (`KismetMathLibrary.VSize` NormalImpulse)) 600.0)))

(event `self.SheildBroken`
  (if (`self.isSheild`)
    (set `self.isSheild` false)
    (`LegacyCameraShake.StartLegacyCameraShake` (`GameplayStatics.GetPlayerCameraManager` 0) "/Game/N_game/other/thesShake.thesShake_C" 10.0)))

(event `self.TheEternal.OnComponentBeginOverlap`
  (params (OverlappedComponent :type "PrimitiveComponent Object Reference") (OtherActor :type "Actor Object Reference") (OtherComp :type "PrimitiveComponent Object Reference") (OtherBodyIndex :type Integer) (bFromSweep :type Boolean) (SweepResult :type "HitResult Structure (by ref)"))
  (if (and (<= (`self.SH_Process`) 0.2) (`GameplayStatics.ObjectIsA` OtherActor "/Game/N_game/BP/OtherBall_Base.OtherBall_Base_C") (not (`self.isSheild`)))
    (bind _asother_ball_base (cast `/Game/N_game/BP/OtherBall_Base` OtherActor))
    (bind _theball (`gameBall.theBall` _asother_ball_base))
    (bind _returnvalue (- (`SceneComponent.K2_GetComponentLocation` _theball) (`SceneComponent.K2_GetComponentLocation` (`self.Sphere`))))
    (`PrimitiveComponent.AddImpulse` _theball (* (`KismetMathLibrary.Normal` _returnvalue) (/ 500000000.0 (`KismetMathLibrary.VSize` _returnvalue))) "None" false)
    (`/Game/N_game/BP/OtherBall_Base.broken` _asother_ball_base)))

(fn `ChosenCheck`
  (bind _thechosenball (`self.theChosenBall`))
  (bind _cherger_0 (`self.Cherger_0`))
  (bind _thechosenball_2 (`self.theChosenBall`))
  (bind _cherger_0_2 (`self.Cherger_0`))
  (`/Engine/EditorBlueprintResources/StandardMacros.IsValid` _thechosenball
    (:`Is Valid`
      (`SceneComponent.K2_SetRelativeLocation` _cherger_0_2 (`KismetMathLibrary.VLerp` (`SceneComponent.RelativeLocation` _cherger_0_2) (50.0 0.0 0.0) 0.2) false false)
      (if (not (== _thechosenball (`self.theLastChosen`)))
        (`SceneComponent.K2_AttachToComponent` (`self.Cherger_0`) (`gameBall.theBall` _thechosenball_2) "None" "KeepWorld" "KeepRelative" "KeepRelative" true)
        (set `self.theLastChosen` _thechosenball_2)))
    (:`Is Not Valid`
      (`SceneComponent.K2_SetRelativeLocation` _cherger_0 (`KismetMathLibrary.VLerp` (`SceneComponent.RelativeLocation` _cherger_0) (50.0 0.0 0.0) 0.2) false false)
      (`SceneComponent.K2_AttachToComponent` (`self.Cherger_0`) (`self.Sphere`) "None" "KeepWorld" "KeepRelative" "KeepRelative" true))))

(fn `SheildProcess`
  (params (dTime :type "Float (double-precision)"))
  (bind _sh_process (`self.SH_Process`))
  (bind _sh_process_2 (`self.SH_Process`))
  (bind _returnvalue (+ (`KismetMathLibrary.Square` (* _sh_process 30.0)) 1.0))
  (`|ExecutionSequence`
    (:`then_0`
      (if (`self.isSheild`)
        (set `self.SH_Process` (`KismetMathLibrary.FMax` (- _sh_process_2 dTime)))
        (else
          (set `self.SH_Process` (`KismetMathLibrary.FMin` (+ _sh_process_2 dTime) 0.5)))))
    (:`then_1`
      (`SceneComponent.SetWorldScale3D` (`self.TheEternal`) (`KismetMathLibrary.MakeVector` _returnvalue _returnvalue _returnvalue)))
    (:`then_2`
      (`MaterialInstanceDynamic.SetScalarParameterValue` (`self.theMat`) "Opa" (- 1.0 (* _sh_process 5.0))))
    (:`then_3`
      (if (and (`self.SheildBack`) (>= _sh_process 0.5))
        (set `self.SheildBack` false)
        (set `self.isSheild` true)
        (`KismetSystemLibrary.PrintText` "Hello")))))

(fn `start`
  (`EnhancedInputSubsystemInterface.AddMappingContext` (pcsubsystem `EnhancedInputLocalPlayerSubsystem` (`GameplayStatics.GetPlayerController` 0)) "/Game/N_game/input/Ball_Input.Ball_Input" 0 (struct))
  (bind _returnvalue (`KismetMaterialLibrary.CreateDynamicMaterialInstance` "/Game/_hl/_common/mat/Eternal_Building.Eternal_Building"))
  (bind _output_get (set `self.theMat` _returnvalue))
  (`PrimitiveComponent.SetMaterial` (`self.TheEternal`) 0 _output_get)
  (`SceneComponent.K2_SetWorldLocation` (`self.Camera`) (5000.0 0.0 0.0) false false)
  (set `self.Cherger_0` (`self.cherger`))
  (bind _returnvalue_2 (`|CreateWidget` "/Game/N_game/UI/theBoard.theBoard_C"))
  (set `self.theBoard` _returnvalue_2)
  (`UserWidget.AddToViewport` _returnvalue_2 0))

(fn `UserConstructionScript`)