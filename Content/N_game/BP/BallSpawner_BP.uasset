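; Spawner actor that creates OtherBall_Base balls at locations passed to its SpawnBall event.
; Spawning adjusts position to avoid collisions and skips the spawn if the spot stays blocked.
; BoxDraw outlines a SpawnAreaX by SpawnAreaY rectangle on the world YZ plane at X=1 with persistent debug line traces, but nothing calls it.
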(event `self.ReceiveBeginPlay`)

(event `self.ReceiveTick`
  (params (DeltaSeconds :type "Float (single-precision)")))

(event `self.SpawnBall`
  (params (spawnLocation :type "Vector Structure"))
  (`|SpawnActorFromClass` "/Game/N_game/BP/OtherBall_Base.OtherBall_Base_C" (`KismetMathLibrary.Conv_VectorToTransform` spawnLocation) "AdjustIfPossibleButDontSpawnIfColliding" "MultiplyWithRoot" null null))

(fn `BoxDraw`
  (bind _returnvalue (/ (`self.SpawnAreaX`) 2.0))
  (bind _returnvalue_2 (/ (`self.SpawnAreaY`) 2.0))
  (bind _returnvalue_3 (* _returnvalue -1.0))
  (bind _returnvalue_4 (* _returnvalue_2 -1.0))
  (`KismetSystemLibrary.LineTraceSingle` :`Start` (`KismetMathLibrary.MakeVector` 1.0 _returnvalue _returnvalue_2) :`End` (`KismetMathLibrary.MakeVector` 1.0 _returnvalue _returnvalue_4) :`TraceChannel` "TraceTypeQuery1" :`DrawDebugType` "Persistent" :`TraceColor` (struct :`G` 1.0 :`A` 1.0))
  (`KismetSystemLibrary.LineTraceSingle` :`Start` (`KismetMathLibrary.MakeVector` 1.0 _returnvalue _returnvalue_2) :`End` (`KismetMathLibrary.MakeVector` 1.0 _returnvalue_3 _returnvalue_2) :`TraceChannel` "TraceTypeQuery1" :`DrawDebugType` "Persistent" :`TraceColor` (struct :`G` 1.0 :`A` 1.0))
  (`KismetSystemLibrary.LineTraceSingle` :`Start` (`KismetMathLibrary.MakeVector` 1.0 _returnvalue_3 _returnvalue_4) :`End` (`KismetMathLibrary.MakeVector` 1.0 _returnvalue _returnvalue_4) :`TraceChannel` "TraceTypeQuery1" :`DrawDebugType` "Persistent" :`TraceColor` (struct :`G` 1.0 :`A` 1.0))
  (`KismetSystemLibrary.LineTraceSingle` :`Start` (`KismetMathLibrary.MakeVector` 1.0 _returnvalue_3 _returnvalue_4) :`End` (`KismetMathLibrary.MakeVector` 1.0 _returnvalue_3 _returnvalue_2) :`TraceChannel` "TraceTypeQuery1" :`DrawDebugType` "Persistent" :`TraceColor` (struct :`G` 1.0 :`A` 1.0)))

(fn `UserConstructionScript`)